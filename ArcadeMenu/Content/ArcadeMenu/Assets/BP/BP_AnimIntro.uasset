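; Arcade menu intro actor that animates a logo, game title and "press start" text on BeginPlay.
; Timelines drive dynamic material parameters to reveal two logo material slots, then slide the title from an offset position back to its placed location.
; After a fixed delay, another timeline drives the press-start text's fade parameter.
; The construction script exposes text, title font size and element offsets for editor tuning.
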(event `self.ReceiveBeginPlay`
  (bind _logo (`self.Logo`))
  (bind _game_name (`self.Game Name`))
  (bind _press_start_name (`self.Press Start Name`))
  ;[1 1 1] Intro Animation
  (bind _output_get (set `self.StartLocation` (`SceneComponent.K2_GetComponentLocation` _game_name)))
  (bind _output_get_2 (set `self.FullOffset` (- _output_get (`self.OffsetForAnimation`))))
  (`SceneComponent.K2_SetWorldLocation` _game_name _output_get_2 false false)
  (`|ExecutionSequence`
    (:`then_0`
      (bind _returnvalue (`PrimitiveComponent.CreateDynamicMaterialInstance` _logo 0 (`PrimitiveComponent.GetMaterial` _logo 0) "None"))
      (`PrimitiveComponent.SetMaterial` _logo 0 _returnvalue)
      (bind (_direction _newtrack_0) (`Timeline|Timeline_0`)
        (:`Update`
          (`MaterialInstanceDynamic.SetScalarParameterValue` _returnvalue "Visability" _newtrack_0))))
    (:`then_1`
      (bind _returnvalue_2 (`PrimitiveComponent.CreateDynamicMaterialInstance` _logo 2 (`PrimitiveComponent.GetMaterial` _logo 2) "None"))
      (`PrimitiveComponent.SetMaterial` _logo 2 _returnvalue_2)
      (bind (_direction_2 _newtrack_0_2) (`Timeline|Timeline_1`)
        (:`Update`
          (`MaterialInstanceDynamic.SetScalarParameterValue` _returnvalue_2 "Visability" _newtrack_0_2))
        (:`Finished`
          (`KismetSystemLibrary.PrintString` "Anim Done")
          (bind (_direction_3 _newtrack_0_3) (`Timeline|Timeline_2`)
            (:`Update`
              (`SceneComponent.K2_SetWorldLocation` (`self.Game Name`) (`KismetMathLibrary.VLerp` (`self.FullOffset`) (`self.StartLocation`) _newtrack_0_3) false false))))))
    (:`then_2`
      (bind _returnvalue_3 (`PrimitiveComponent.CreateDynamicMaterialInstance` _press_start_name 0 (`PrimitiveComponent.GetMaterial` _press_start_name 0) "None"))
      (`PrimitiveComponent.SetMaterial` _press_start_name 0 _returnvalue_3)
      (`KismetSystemLibrary.Delay` 9.0)
      (bind (_direction_4 _newtrack_0_4) (`Timeline|Timeline_3`)
        (:`Update`
          (`MaterialInstanceDynamic.SetScalarParameterValue` _returnvalue_3 "FadeInOut" _newtrack_0_4))))))

(fn `UserConstructionScript`
  (bind _game_name (`self.Game Name`))
  ;[1 1 1] Change Settings from editor
  (`TextRenderComponent.K2_SetText` (`self.Game Name`) (`self.GameName`))
  (`TextRenderComponent.K2_SetText` (`self.Press Start Name`) (`self.Start Game Name`))
  (`SceneComponent.K2_SetRelativeLocation` _game_name (`self.Logo Offset`) false false)
  (`TextRenderComponent.SetWorldSize` _game_name (`self.FontSize`))
  (`SceneComponent.K2_SetRelativeLocation` (`self.Press Start Name`) (`self.Start Game Offset`) false false))