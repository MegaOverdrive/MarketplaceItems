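; Jump pad that launches the Player_JumpingPlatform character toward a linked landing actor when it overlaps the trigger sphere.
; Launch velocity comes from a suggested custom-arc projectile solve aimed slightly above the landing, overriding the character's velocity.
; BeginPlay and the construction script yaw the button mesh toward the landing and pass it to the particle system.
; The construction script also applies its ShowDebugInGame setting to particle visibility on every platform in the level.
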(event `self.ReceiveBeginPlay`
  (bind _landing_reference (`self.Landing Reference`))
  ;[1 1 1] Update Rotation
  (`ParticleSystemComponent.SetActorParameter` (`self.ParticleSystem`) "BP_Landing" _landing_reference)
  (`SceneComponent.K2_SetRelativeRotation` (`self.JumpPlatform_SM_Button`) (`KismetMathLibrary.MakeRotator` 0.0 0.0 (.yaw (`KismetMathLibrary.FindLookAtRotation` (`self.K2_GetActorLocation`) (`self.K2_GetActorLocation` _landing_reference)))) false false))

(event `self.Sphere.OnComponentBeginOverlap`
  (params (OverlappedComponent :type "PrimitiveComponent Object Reference") (OtherActor :type "Actor Object Reference") (OtherComp :type "PrimitiveComponent Object Reference") (OtherBodyIndex :type Integer) (bFromSweep :type Boolean) (SweepResult :type "HitResult Structure (by ref)"))
  ;[1 1 1] LaunchPlayer
  (bind _asplayer_jumping_platform (cast `/Game/JumpPlatform/Player/Blueprints/Player_JumpingPlatform` OtherActor)) ; Switch This to your player
  (bind _outlaunchvelocity (`GameplayStatics.SuggestProjectileVelocity_CustomArc` (`self.K2_GetActorLocation` _asplayer_jumping_platform) (+ (`self.K2_GetActorLocation` (`self.Landing Reference`)) (0.0 0.0 80.0)) 0.0 0.6))
  (`Character.LaunchCharacter` _asplayer_jumping_platform _outlaunchvelocity true true))

(fn `UserConstructionScript`
  (bind _particlesystem (`self.ParticleSystem`))
  (bind _landing_reference (`self.Landing Reference`))
  ;[1 1 1] Update Rotation
  (set `self.Update Arrow Rotation` true)
  (set `self.Update Arrow Rotation` false)
  (bind _outactors (`GameplayStatics.GetAllActorsOfClass` "BP_JumpPlatform_C"))
  (for _array_element _outactors
    (if (`self.Show Debug in Game`)
      (`SceneComponent.SetHiddenInGame` _particlesystem false false)
      (`SceneComponent.SetHiddenInGame` (`/Game/JumpPlatform/BP_JumpPlatform.ParticleSystem` _array_element) false false)
      (else
        (`SceneComponent.SetHiddenInGame` _particlesystem true false)
        (`SceneComponent.SetHiddenInGame` (`/Game/JumpPlatform/BP_JumpPlatform.ParticleSystem` _array_element) true false)))
    (`ParticleSystemComponent.SetActorParameter` (`self.ParticleSystem`) "BP_Landing" _landing_reference)
    (`SceneComponent.K2_SetRelativeRotation` (`self.JumpPlatform_SM_Button`) (`KismetMathLibrary.MakeRotator` 0.0 0.0 (.yaw (`KismetMathLibrary.FindLookAtRotation` (`self.K2_GetActorLocation`) (`self.K2_GetActorLocation` _landing_reference)))) false false)))